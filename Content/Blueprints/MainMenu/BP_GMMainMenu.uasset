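; Main menu game mode that starts the UI and handles hosting and finding multiplayer sessions.
; On BeginPlay it has the first player's menu controller set up UI and player data.
; Hosting uses an Advanced Sessions node, then has the game instance load the game level on success.
; Finding searches all server types and asks the game instance to join every result in turn, with no selection or filtering.
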(event Custom|HostGameSession
  (params (InPlayerController :type Player%20Controller%20Object%20Reference))
  (|AdvancedSession 0 InPlayerController 100 0 false true false true true true false false false true
    (:OnSuccess
      (bind _asbp_game_instance (Utilities|Casting|CastToBP_GameInstance (Game|GetGameInstance)))
      (Default|LoadGameLevel _asbp_game_instance (Variables|Default|GetGameLevel)))))

(event Custom|FindGameSessions
  (params (PlayerController :type Player%20Controller%20Object%20Reference))
  (bind _results (|FindSessionsAdvanced PlayerController 0 false "AllServers" 0 false false false true)
    (:OnSuccess
      (for _array_element _results
        (bind _asbp_game_instance (Utilities|Casting|CastToBP_GameInstance (Game|GetGameInstance)))
        (Default|JoinGameSession _asbp_game_instance _array_element PlayerController)))))

(event EventBeginPlay
  (bind _asbp_mmplayer_controller (Utilities|Casting|CastToBP_MMPlayerController (Game|GetPlayerController 0)))
  (Default|SetUIandPlayerData _asbp_mmplayer_controller))

(event EventTick
  (params (DeltaSeconds :type Float%20%28single-precision%29)))

(fn ConstructionScript)