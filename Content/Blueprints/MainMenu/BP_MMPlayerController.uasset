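; Main menu player controller that sets up the menu UI and player data.
; SetUIAndPlayerData creates the main menu widget, passes it the player's save, switches to UI-only input and copies the saved player data into the game instance.
; GetPlayerDataSave loads the options save from the game instance's slot, or creates and saves a new one if none exists.
; Key 1 prints a debug greeting.
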(event Custom|SetUIAndPlayerData
  (bind _asbp_player_options_save_game (CallFunction|GetPlayerDataSave))
  (bind _returnvalue (UserInterface|CreateWidget "/Game/Blueprints/MainMenu/UW_MainMenu.UW_MainMenu_C" self))
  (bind _output_get (Variables|Default|SetMainMenuWidgetRef _returnvalue))
  (Default|SetupPlayerData _output_get _asbp_player_options_save_game)
  (UserInterface|Viewport|AddtoViewport _output_get 0)
  (Input|SetInputModeUIOnly self _output_get "LockOnCapture")
  (bind _asbp_game_instance (Utilities|Casting|CastToBP_GameInstance (Game|GetGameInstance)))
  (Variables|/Game/Blueprints/BP_GameInstance.BP_GameInstance_C|SetPlayerData _asbp_game_instance (Variables|/Game/Blueprints/MainMenu/BP_PlayerOptions_SaveGame.BP_PlayerOptions_SaveGame_C|GetPlayerData _asbp_player_options_save_game)))

(event EventBeginPlay)

(event EventTick
  (params (DeltaSeconds :type Float%20%28single-precision%29)))

(event Input|KeyboardEvents|1
  (params (Key :type Key%20Structure :default "None"))
  (:Pressed
    (Development|PrintString "Hello")))

(fn ConstructionScript)

(fn GetPlayerDataSave
  (bind _output_get (LocalVariables|SetSaveGameSlotName (Variables|/Script/GEM.GEMGameInstance|GetSaveGameSlot (Class|GEMBlueprintFunctionLibrary|GetGEMGameInstance))))
  (bind _returnvalue (SaveGame|DoesSaveGameExist _output_get))
  (if _returnvalue
    (bind _returnvalue_2 (SaveGame|LoadGamefromSlot (LocalVariables|GetSaveGameSlotName)))
    (bind _asbp_player_options_save_game (Utilities|Casting|CastToBP_PlayerOptions_SaveGame _returnvalue_2))
    (return _asbp_player_options_save_game)
    (else
      (bind _returnvalue_3 (Game|ConstructObjectfromClass "/Game/Blueprints/MainMenu/BP_PlayerOptions_SaveGame.BP_PlayerOptions_SaveGame_C" self))
      (SaveGame|SaveGametoSlot _returnvalue_3 (LocalVariables|GetSaveGameSlotName))
      (return _returnvalue_3))))