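; BP_MoveablePlatform is a platform that moves along a spline while tagged actors overlap its collision, and returns when the last one leaves.
; Server-only overlap events check a required tag and track occupants in an array, then trigger movement after a short delay.
; A timeline, noted as replicated to clients and rate-scaled by TravelDuration, plays or reverses to place the mesh by distance along the spline.
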(event OnComponentBeginOverlap(CollisionOverlap)
  (params (OverlappedComponent :type Primitive%20Component%20Object%20Reference) (OtherActor :type Actor%20Object%20Reference) (OtherComp :type Primitive%20Component%20Object%20Reference) (OtherBodyIndex :type Integer) (bFromSweep :type Boolean) (SweepResult :type Hit%20Result%20Structure%20%28by%20ref%29))
  ;[0.1121 0.1281 1] Overlap Events - Checks to see if a valid actor is added or removed on the server and moves the spine
  (Networking|SwitchHasAuthority
    (:Authority
      (Utilities|CheckActorTag OtherActor (Variables|Default|GetRequiredTag)
        (:HasTag
          (Utilities|Array|Add (Variables|Default|GetOverlappedActors) OtherActor)
          (CallFunction|MoveAlongSpline true))))))

(event OnComponentEndOverlap(CollisionOverlap)
  (params (OverlappedComponent :type Primitive%20Component%20Object%20Reference) (OtherActor :type Actor%20Object%20Reference) (OtherComp :type Primitive%20Component%20Object%20Reference) (OtherBodyIndex :type Integer))
  ;[0.1121 0.1281 1] Overlap Events - Checks to see if a valid actor is added or removed on the server and moves the spine
  (Networking|SwitchHasAuthority
    (:Authority
      (Utilities|CheckActorTag OtherActor (Variables|Default|GetRequiredTag)
        (:HasTag
          (Utilities|Array|RemoveItem (Variables|Default|GetOverlappedActors) OtherActor)
          (if (Class|GEMBlueprintFunctionLibrary|ArrayIsEmpty (Variables|Default|GetOverlappedActors))
            (CallFunction|MoveAlongSpline false)))))))

(event Custom|MoveAlongSpline
  (params (bCanMoveForward :type Boolean))
  (bind _spline (Variables|Default|GetSpline))
  ;[1 0.1476 0.6953] Run on Server - Timeline is replicated to clients
  (Utilities|FlowControl|Delay 0.5)
  (if bCanMoveForward
    (bind _alpha (Timeline|MovePlatform Play)
      (:Update
        (Transformation|SetWorldLocation (Variables|Default|GetStaticMesh) (Spline|GetLocationatDistanceAlongSpline _spline (Math|Float|Lerp 0.0 (Spline|GetSplineLength _spline) _alpha) "World") false false)))
    (else
      (Timeline|MovePlatform Reverse))))

(event EventBeginPlay
  ;[1 1 1] Set how long duration of timeline is
  (Components|Timeline|SetPlayRate (Variables|Default|GetMovePlatform) (/ 1.0 (Variables|Default|GetTravelDuration))))

(fn ConstructionScript)