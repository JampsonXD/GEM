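; BP_Key_activity_4_end is an Hour of Code key pickup that grants a key to a player who does not already hold one.
; On the server, a sphere overlap by a correctly tagged actor sets the Key flag on its controller's BP_GEMPS player state.
; A multicast then hides the actor and plays the pickup sound only for the collecting player's local controller.
; The key destroys itself after a short delay.
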(event OnComponentBeginOverlap(Sphere_coll)
  (params (OverlappedComponent :type Primitive%20Component%20Object%20Reference) (OtherActor :type Actor%20Object%20Reference) (OtherComp :type Primitive%20Component%20Object%20Reference) (OtherBodyIndex :type Integer) (bFromSweep :type Boolean) (SweepResult :type Hit%20Result%20Structure%20%28by%20ref%29))
  (bind _returnvalue (Game|GetInstigatorController OtherActor))
  ;[0.08689 0.1596 1] Overlap Event
  (Networking|SwitchHasAuthority
    (:Authority
      (Utilities|CheckActorTag OtherActor (Variables|Default|GetTagName)
        (:HasTag
          ;;[0.09807 0.789 1] Check if the player already has a key
          (bind _asbp_gemps (Utilities|Casting|CastToBP_GEMPS (Variables|/Script/Engine.Controller|GetPlayerState _returnvalue)))
          (if (not (Variables|/Game/Blueprints/Game/BP_GEMPS.BP_GEMPS_C|GetKey _asbp_gemps))
            (Variables|/Game/Blueprints/Game/BP_GEMPS.BP_GEMPS_C|SetKey _asbp_gemps true)
            (CallFunction|MultiCastSFX _returnvalue)
            (CallFunction|OnUsed)))))))

(event Custom|MultiCast_SFX
  (params (InController :type Controller%20Object%20Reference))
  ;[1 0.05018 0.02034] Play Sound for player that picks up Key, and change their HUD
  (Utilities|FlowControl|Sequence
    (:then_0
      (if (Class|GEMBlueprintFunctionLibrary|IsControllerLocal InController)
        (Audio|PlaySound2D "/Game/Assets/Hour_of_Code/Audio/SFX_key.SFX_key" 1.0 1.0 0.0 0 0)))
    (:then_1
      ;;[1 1 1] Hide Actor for all nearby players on use
      (Rendering|SetActorHiddenInGame true))))

(event Custom|OnUsed
  ;[1 1 1] Functionality after the object has been used
  (Utilities|FlowControl|Delay 0.25)
  (Actor|DestroyActor))

(fn ConstructionScript)