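; Game mode that initializes each joining player and assigns their starting spawn transform, with seamless travel enabled in the construction script.
; On PostLogin it sets game-only input, then calls client player data setup on the BP_GEMPlayerController and hands it the spawn transform.
; That transform uses only the location of the first PlayerStart found, with zero rotation and unit scale, so every player receives the same start.
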(event EventPostLogin
  (params (NewPlayer :type Player%20Controller%20Object%20Reference))
  ;[1 1 1] Set Spawn Location and Create HUD on login
  (Input|SetInputModeGameOnly NewPlayer)
  (bind _asbp_gemplayer_controller (Utilities|Casting|CastToBP_GEMPlayerController NewPlayer))
  (Default|ClientSetupPlayerData _asbp_gemplayer_controller)
  (bind _returnvalue (CallFunction|SetStartingSpawnLocation))
  (Class|GEMPlayerController|SetSpawnTransform _asbp_gemplayer_controller _returnvalue))

(event EventTick
  (params (DeltaSeconds :type Float%20%28single-precision%29)))

(fn ConstructionScript
  (Variables|Default|SetbUseSeamlessTravel true))

(fn SetStartingSpawnLocation
  (bind _outactors (Actor|GetAllActorsOfClass "/Script/Engine.PlayerStart"))
  (return (Math|Transform|MakeTransform (.Location (Math|Transform|BreakTransform (Transformation|GetActorTransform (Utilities|Array|Get(acopy) _outactors)))) "0, 0, 0" "1,1,1")))