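; Weapon pickup that grants an overlapping GEMCharacter a random weapon from a data asset list, added to inventory without equipping it.
; Construction script picks the first weapon and sets its mesh and first attachment; a looping timer spins it while off cooldown.
; Cooldown hides the weapon mesh while the server async-loads a new random weapon, then refreshes both meshes when it ends.
; The interacting local player hears a pickup sound.
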(event Custom|RotateMesh
  ;[0.1667 0.1667 0.1667] Rotate Mesh at a Constant Tickrate
  (if (not (Variables|Default|GetbCooldownActive))
    (Transformation|AddRelativeRotation (Variables|Default|GetWeaponMesh) (Math|Rotator|MakeRotator 0.0 0.0 (Variables|Default|GetRotationValue)) false false)))

(event EventTick
  (params (DeltaSeconds :type Float%20%28single-precision%29))
  (|CallParentFunction DeltaSeconds))

(event EventOnCooldownSet
  (params (IsCooldownOn :type Boolean))
  (bind _weaponmesh (Variables|Default|GetWeaponMesh))
  ;[0.1667 0.1667 0.1667] Cooldown Functionality
  (|CallParentFunction IsCooldownOn)
  (Rendering|SetVisibility (Variables|Default|GetWeaponMesh) (not IsCooldownOn) false)
  (if IsCooldownOn
    ;;[1 1 1] Sets a new random weapon from our Array to give the player - Server only
    (Networking|SwitchHasAuthority
      (:Authority
        (bind _object (Utilities|AsyncLoadAsset (.OutItem (Utilities|Array|Random (Variables|Default|GetWeapon%20DA%20List))))
          (:then
            (bind _asgemweapon_data (Utilities|Casting|CastToGEMWeaponData _object))
            (Variables|Default|SetWeapon%20DA _asgemweapon_data)))))
    (else
      (Class|SkinnedMeshComponent|SetSkeletalMesh _weaponmesh (.skeletalmesh (Variables|/Script/GEM.GEMWeaponData|GetWeaponMesh (Variables|Default|GetWeapon%20DA))) true)
      (Transformation|AttachComponentToComponent (Variables|Default|GetScope) _weaponmesh (.SocketAttachName (Utilities|Struct|BreakSubWeaponMeshData (Utilities|Array|Get(acopy) (Variables|/Script/GEM.GEMWeaponData|GetAttachmentMeshes (Variables|Default|GetWeapon%20DA))))) "SnapToTarget" "SnapToTarget" "SnapToTarget" true)
      (Class|SkinnedMeshComponent|SetSkeletalMesh (Variables|Default|GetScope) (.SkeletalMesh (Utilities|Struct|BreakSubWeaponMeshData (Utilities|Array|Get(acopy) (Variables|/Script/GEM.GEMWeaponData|GetAttachmentMeshes (Variables|Default|GetWeapon%20DA))))) true))))

(event EventPlayEffects
  (params (InInstigatingController :type Controller%20Object%20Reference))
  ;[1 1 1] On Interact Effects
  ;[0.1667 0.1667 0.1667] Cooldown Functionality
  (|CallParentFunction InInstigatingController)
  (if (Class|GEMBlueprintFunctionLibrary|IsControllerLocal InInstigatingController)
    (Audio|PlaySound2D "/Game/Sounds/InterfaceAndItemSounds/Cues/Special_Musical_02_wav_Cue.Special_Musical_02_wav_Cue" 1.0 1.0 0.0 0 0)))

(event EventOverlapEvent
  (params (InActor :type Actor%20Object%20Reference))
  ;[1 1 1] Overlap Event Functionality
  (bind _asgemcharacter (Utilities|Casting|CastToGEMCharacter InActor))
  (Class|GEMCharacter|AddWeapontoInventory _asgemcharacter (Utilities|Struct|MakeInventoryWeaponData (Variables|Default|GetWeapon%20DA) 0 -1) false))

(event EventBeginPlay
  ;[0.1667 0.1667 0.1667] Rotate Mesh at a Constant Tickrate
  (|CallParentFunction)
  (Utilities|Time|SetTimerbyEvent (EventDispatchers|CreateEvent :!event Custom|RotateMesh) 0.016667 true))

(fn ConstructionScript
  (|CallParentFunction)
  (bind _returnvalue (Utilities|LoadAssetBlocking (.OutItem (Utilities|Array|Random (Variables|Default|GetWeapon%20DA%20List)))))
  (bind _asgemweapon_data (Utilities|Casting|CastToGEMWeaponData _returnvalue))
  (bind _output_get (Variables|Default|SetWeapon%20DA _asgemweapon_data))
  (Class|SkinnedMeshComponent|SetSkeletalMesh (Variables|Default|GetWeaponMesh) (.skeletalmesh (Variables|/Script/GEM.GEMWeaponData|GetWeaponMesh _output_get)) true)
  (Transformation|AttachComponentToComponent (Variables|Default|GetScope) (Variables|Default|GetWeaponMesh) (.SocketAttachName (Utilities|Struct|BreakSubWeaponMeshData (Utilities|Array|Get(acopy) (Variables|/Script/GEM.GEMWeaponData|GetAttachmentMeshes (Variables|Default|GetWeapon%20DA))))) "SnapToTarget" "SnapToTarget" "SnapToTarget" true)
  (Class|SkinnedMeshComponent|SetSkeletalMesh (Variables|Default|GetScope) (.SkeletalMesh (Utilities|Struct|BreakSubWeaponMeshData (Utilities|Array|Get(acopy) (Variables|/Script/GEM.GEMWeaponData|GetAttachmentMeshes (Variables|Default|GetWeapon%20DA))))) true))