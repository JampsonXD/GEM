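; BP_JumpBoostPU is a jump boost pickup that temporarily raises a BP_SuperCharacter's jump velocity.
; It extends a parent powerup's overlap, effects and cooldown events, adding JumpVelocityAdditive on overlap and storing the character to subtract it when the cooldown finishes.
; The powerup mesh hides during cooldown, and the multicast effects event plays the boost sound only for the locally controlled instigator.
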(event EventBeginPlay
  (|CallParentFunction) ; This node is disabled and will not be called.\nDrag off pins to build functionality.
)

(event Collision|EventActorBeginOverlap
  (params (OtherActor :type Actor%20Object%20Reference))
  (|CallParentFunction OtherActor) ; This node is disabled and will not be called.\nDrag off pins to build functionality.
)

(event EventTick
  (params (DeltaSeconds :type Float%20%28single-precision%29))
  (|CallParentFunction DeltaSeconds) ; This node is disabled and will not be called.\nDrag off pins to build functionality.
)

(event EventOverlapEvent
  (params (InActor :type Actor%20Object%20Reference))
  ;[1 1 1] Overlap Event
  (|CallParentFunction InActor)
  (bind _asbp_super_character (Utilities|Casting|CastToBP_SuperCharacter InActor))
  (bind _output_get (Variables|Default|SetAs%20Third%20Person%20Character _asbp_super_character))
  (Variables|/Game/Blueprints/Game/BP_SuperCharacter.BP_SuperCharacter_C|SetJumpVelocity _output_get (+ (Variables|/Game/Blueprints/Game/BP_SuperCharacter.BP_SuperCharacter_C|GetJumpVelocity _output_get) (Variables|Default|GetJumpVelocityAdditive))))

(event EventPlayEffects
  (params (InInstigatingController :type Controller%20Object%20Reference))
  ;[1 1 1] Multicast Play Effects
  (|CallParentFunction InInstigatingController)
  (if (Class|GEMBlueprintFunctionLibrary|IsControllerLocal InInstigatingController)
    (Audio|PlaySoundatLocation "/Game/Assets/Hour_of_Code/Audio/SFX_jump_boost.SFX_jump_boost" (Transformation|GetActorLocation) "0, 0, 0" 1.0 1.0 0.0 0 0 0)))

(event EventOnCooldownSet
  (params (IsCooldownOn :type Boolean))
  ;[1 1 1] Cooldown Changed
  (|CallParentFunction IsCooldownOn)
  (Rendering|SetVisibility (Variables|Default|GetSM_powerup) (not IsCooldownOn) false))

(event EventCooldownFinished
  ;[1 1 1] Cooldown Finished
  (Utilities|IsValid (Variables|Default|GetAs%20Third%20Person%20Character)
    (:Is%20Valid
      (Variables|/Game/Blueprints/Game/BP_SuperCharacter.BP_SuperCharacter_C|SetJumpVelocity (Variables|Default|GetAs%20Third%20Person%20Character) (- (Variables|/Game/Blueprints/Game/BP_SuperCharacter.BP_SuperCharacter_C|GetJumpVelocity (Variables|Default|GetAs%20Third%20Person%20Character)) (Variables|Default|GetJumpVelocityAdditive)))
      (Variables|Default|SetAs%20Third%20Person%20Character 0))))

(fn ConstructionScript
  (|CallParentFunction))