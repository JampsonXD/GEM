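; BP_HealthPU is a health pickup that extends a parent pickup class and only triggers for actors whose health is not full.
; On overlap it applies GE_HealthPickup through the actor's Ability System Component, passing HealthToAdd as a SetByCaller magnitude.
; It plays a 2D sound only for a locally controlled instigator and hides its NSPickup3 visual while on cooldown.
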(event EventBeginPlay
  (|CallParentFunction) ; This node is disabled and will not be called.\nDrag off pins to build functionality.
)

(event Collision|EventActorBeginOverlap
  (params (OtherActor :type Actor%20Object%20Reference))
  (|CallParentFunction OtherActor) ; This node is disabled and will not be called.\nDrag off pins to build functionality.
)

(event EventTick
  (params (DeltaSeconds :type Float%20%28single-precision%29))
  (|CallParentFunction DeltaSeconds) ; This node is disabled and will not be called.\nDrag off pins to build functionality.
)

(event EventOverlapEvent
  (params (InActor :type Actor%20Object%20Reference))
  (bind _returnvalue (Ability|GetAbilitySystemComponent InActor))
  (|CallParentFunction InActor)
  (bind _returnvalue_2 (Ability|GameplayEffect|AssignTagSetbyCallerMagnitude (GameplayEffects|MakeOutgoingSpec _returnvalue "/Game/Blueprints/Game/GE/Misc/GE_HealthPickup.GE_HealthPickup_C" 0.0 (GameplayEffects|MakeEffectContext _returnvalue)) "(TagName=\"Data.Value1\")" (Variables|Default|GetHealthToAdd)))
  (GameplayEffects|ApplyGameplayEffectSpecToSelf _returnvalue _returnvalue_2))

(event EventPlayEffects
  (params (InInstigatingController :type Controller%20Object%20Reference))
  (|CallParentFunction InInstigatingController)
  (if (Class|GEMBlueprintFunctionLibrary|IsControllerLocal InInstigatingController)
    (Audio|PlaySound2D "/Game/Sounds/InterfaceAndItemSounds/Cues/Special_Musical_02_wav_Cue.Special_Musical_02_wav_Cue" 1.0 1.0 0.0 0 0)))

(event EventOnCooldownSet
  (params (IsCooldownOn :type Boolean))
  (|CallParentFunction IsCooldownOn)
  (Rendering|SetVisibility (Variables|Default|GetNS_Pickup_3) (not IsCooldownOn) false))

(fn ConstructionScript
  (|CallParentFunction))

(fn CanTriggerEvent
  (params (InActor :type Actor%20Object%20Reference))
  (bind _returnvalue (|CallParentFunction InActor))
  (return (and _returnvalue (not (CallFunction|IsHealthFull InActor)))))

(fn IsHealthFull
  (params (InActor :type Actor%20Object%20Reference))
  (bind _returnvalue (Ability|GetAbilitySystemComponent InActor))
  (return (== (.ReturnValue (Ability|Attribute|GetFloatAttributefromAbilitySystemComponent _returnvalue "(AttributeName=\"Health\",Attribute=/Script/GEM.GEMAttributeSetBase:Health,AttributeOwner=None)")) (.ReturnValue (Ability|Attribute|GetFloatAttributefromAbilitySystemComponent _returnvalue "(AttributeName=\"MaxHealth\",Attribute=/Script/GEM.GEMAttributeSetBase:MaxHealth,AttributeOwner=None)")))))