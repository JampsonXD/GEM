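; Coin pickup that extends a parent pickup and grants coins to the overlapping actor through the Gameplay Ability System.
; On overlap it applies GE_Coins to that actor's ASC, passing CoinAmount as a set-by-caller magnitude.
; The multicast effects event plays the coin sound only for the locally controlled instigator and hides the pickup.
; Post-overlap delays briefly before destroying the actor.
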(event EventBeginPlay
  (|CallParentFunction) ; This node is disabled and will not be called.\nDrag off pins to build functionality.
)

(event Collision|EventActorBeginOverlap
  (params (OtherActor :type Actor%20Object%20Reference))
  (|CallParentFunction OtherActor) ; This node is disabled and will not be called.\nDrag off pins to build functionality.
)

(event EventTick
  (params (DeltaSeconds :type Float%20%28single-precision%29))
  (|CallParentFunction DeltaSeconds) ; This node is disabled and will not be called.\nDrag off pins to build functionality.
)

(event EventOverlapEvent
  (params (InActor :type Actor%20Object%20Reference))
  ;[1 1 1] Overlap Event
  (|CallParentFunction InActor)
  (CallFunction|AddCoins InActor))

(event EventPostOverlapEvent
  ;[1 1 1] Post Overlap
  (|CallParentFunction)
  (Utilities|FlowControl|Delay 3.0)
  (Actor|DestroyActor))

(event EventPlayEffects
  (params (InInstigatingController :type Controller%20Object%20Reference))
  ;[1 1 1] Multicast - Effects
  (|CallParentFunction InInstigatingController)
  (Utilities|FlowControl|Sequence
    (:then_0
      (if (Class|GEMBlueprintFunctionLibrary|IsControllerLocal InInstigatingController)
        (Audio|PlaySoundatLocation "/Game/Assets/Hour_of_Code/Audio/SFX_coin.SFX_coin" (Transformation|GetActorLocation (Pawn|GetControlledPawn InInstigatingController)) "0, 0, 0" 1.0 1.0 0.0 0 0 0)))
    (:then_1
      ;;[1 0.1279 0.5541] Hide the Actor for all players neraby before destrouction
      (Rendering|SetActorHiddenInGame true))))

(fn ConstructionScript
  (|CallParentFunction))

(fn AddCoins
  (params (InActor :type Actor%20Object%20Reference))
  (LocalVariables|SetActorASC (Ability|GetAbilitySystemComponent InActor))
  (bind _returnvalue (Ability|GameplayEffect|AssignTagSetbyCallerMagnitude (GameplayEffects|MakeOutgoingSpec (LocalVariables|GetActorASC) "/Game/Blueprints/Game/GE/Misc/GE_Coins.GE_Coins_C" 0.0 (GameplayEffects|MakeEffectContext (LocalVariables|GetActorASC))) "(TagName=\"Data.Value1\")" (Math|Conversions|ToFloat(Integer) (Variables|Default|GetCoin%20Amount))))
  (GameplayEffects|ApplyGameplayEffectSpecToSelf (LocalVariables|GetActorASC) _returnvalue))