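; Player controller for GEM that bridges client and server for player setup, input mapping, interaction and kill events.
; It copies GameInstance player data to the PlayerState, stores the checkpoint, and routes interactions to the target actor through server events.
; Deaths load the killer's character data, asynchronously if needed, for a client HUD recap; kills grant experience through GAS.
; Number keys trigger debug gameplay effects and DLSS switching.
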(event Custom|Client_WasKilled
  (params (EnemyData :type GEM%20Character%20Data%20Object%20Reference))
  (Class|UWHUD|PlayDeathRecap (Class|GEMPlayerController|GetGEMHUD) EnemyData))

(event Custom|Server_ApplyGameplayEffect
  (params (GameplayEffect :type Gameplay%20Effect%20Class%20Reference))
  (GameplayEffects|ApplyGameplayEffectToSelf :self (Ability|GetAbilitySystemComponent (Variables|Default|GetPlayerState)) :GameplayEffectClass GameplayEffect))

(event Custom|Client_SetupPlayerData
  ;[1 0.09796 0.6994] Initial Player Data Setup
  (bind _asbp_game_instance (Utilities|Casting|CastToBP_GameInstance (Game|GetGameInstance)))
  (CallFunction|ServerSendPlayerDatatoPS (Variables|/Game/Blueprints/BP_GameInstance.BP_GameInstance_C|GetPlayerData _asbp_game_instance))
  (if (Class|DLSSLibrary|IsDLSSSupported)
    (Class|DLSSLibrary|SetDLSSMode "Balanced")
    (else
      (Class|DLSSLibrary|SetDLSSMode "Off"))))

(event Custom|Server_SendPlayerDataToPS
  (params (InPlayerData :type Player%20Data%20Structure))
  ;[1 0.09796 0.6994] Initial Player Data Setup
  (Class|INFPlayerState|SetPlayerData(Message) (Variables|Default|GetPlayerState) InPlayerData))

(event Custom|InteractWithInteractingActor
  ;[1 1 1] Interacting with objects, called from outside and sent to server
  (CallFunction|ServerPlayerTryInteract (Variables|Default|GetInteractingActor)))

(event Custom|Client_SetInputMapping
  (params (MappingContext :type Input%20Mapping%20Context%20Object%20Reference) (bClearMappings :type Boolean))
  (bind _self self)
  (bind _returnvalue (PlayerController|LocalPlayerSubsystems|GetEnhancedInputLocalPlayerSubsystem _self))
  ;[0.2517 0.2517 0.2517] Set Mapping Context Passed In - Clear other active mapping contexts if Clear Mappings is True
  (if bClearMappings
    (Class|EnhancedInputSubsystemInterface|ClearAllMappings _returnvalue))
  (Input|AddMappingContext _returnvalue MappingContext 0))

(event Custom|Server_SetCheckpoint
  (params (InCheckpoint :type BP%20Checkpoint%20Object%20Reference))
  ;[1 0.1398 0.07005] Current Checkpoint Reference
  (Variables|Default|SetCurrentCheckpoint InCheckpoint))

(event Custom|Server_PlayerTryInteract
  (params (Actor :type Actor%20Object%20Reference%20%28by%20ref%29))
  ;[1 1 1] Interacting with objects, called from outside and sent to server
  (Class|BPInteractableIF|Interact(Message) Actor self))

(event Custom|PlayerTryInteract
  (params (Actor :type Actor%20Object%20Reference%20%28by%20ref%29))
  ;[1 1 1] Interacting with objects, called from outside and sent to server
  (CallFunction|ServerPlayerTryInteract Actor))

(event Input|EnhancedActionEvents|EnhancedInputActionIA_Confirm
  (params (ActionValue :type Boolean) (ElapsedSeconds :type Float%20%28single-precision%29) (TriggeredSeconds :type Float%20%28single-precision%29))
  (Class|BPInteractableIF|Interact(Message) (Variables|Default|GetInteractingActor) self))

(event Input|EnhancedActionEvents|EnhancedInputActionIA_Cancel
  (params (ActionValue :type Boolean) (ElapsedSeconds :type Float%20%28single-precision%29) (TriggeredSeconds :type Float%20%28single-precision%29))
  (CallFunction|ClientSetInputMapping "/Game/Blueprints/Game/Character/IMC_Default.IMC_Default" true))

(event EventWasKilled
  (params (InKillingPlayer :type GEM%20Character%20Object%20Reference) (bSelfInflicted :type Boolean))
  (bind _returnvalue (Class|GEMCharacter|GetCharacterInfo InKillingPlayer))
  (bind _returnvalue_2 (Class|KismetSystemLibrary|GetObjectfromPrimaryAssetId _returnvalue))
  (Utilities|IsValid _returnvalue_2
    (:Is%20Valid
      _)
    (:Is%20Not%20Valid
      (|AsyncLoadPrimaryAsset _returnvalue
        (:Completed
          _))))
  (bind _asgemcharacter_data (Utilities|Casting|CastToGEMCharacterData _returnvalue_2))
  (CallFunction|ClientWasKilled _asgemcharacter_data))

(event EventKilledCharacter
  (params (InKilledPlayer :type GEM%20Character%20Object%20Reference) (InCharacterLevel :type Float%20%28single-precision%29))
  (bind _returnvalue (Pawn|GetControlledPawn))
  (bind _returnvalue_2 (Ability|GetAbilitySystemComponent _returnvalue))
  (Utilities|IsValid _returnvalue_2
    (:Is%20Valid
      (GameplayEffects|ApplyGameplayEffectToSelf :self _returnvalue_2 :GameplayEffectClass "/Game/Blueprints/Game/GE/Misc/GE_GenericExperience.GE_GenericExperience_C" :Level InCharacterLevel))))

(event Input|KeyboardEvents|3
  (params (Key :type Key%20Structure :default "None"))
  (:Pressed
    (CallFunction|ServerApplyGameplayEffect "/Game/Blueprints/Game/Debug/GE_Debug_ApplyDamage.GE_Debug_ApplyDamage_C")))

(event Input|KeyboardEvents|1
  (params (Key :type Key%20Structure :default "None"))
  (:Pressed
    (CallFunction|ServerApplyGameplayEffect "/Game/Blueprints/Game/Debug/GE_Debug_AddMovementSpeed.GE_Debug_AddMovementSpeed_C")))

(event Input|KeyboardEvents|2
  (params (Key :type Key%20Structure :default "None"))
  (:Pressed
    (CallFunction|ServerApplyGameplayEffect "/Game/Blueprints/Game/Debug/GE_Debug_ReduceMovementSpeed.GE_Debug_ReduceMovementSpeed_C")))

(event Input|KeyboardEvents|4
  (params (Key :type Key%20Structure :default "None"))
  (:Pressed
    (Utilities|FlowControl|FlipFlop
      (:A
        (Class|DLSSLibrary|SetDLSSMode "Off"))
      (:B
        (Class|DLSSLibrary|SetDLSSMode "UltraPerformance")))))

(fn ConstructionScript)