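; Base-style player character built on the Gameplay Ability System, with an overhead healthbar widget, weapon inventory and damage from falls.
; Landing applies a fall damage effect scaled by a curve of Z velocity, while falling out of the world applies instant death.
; Replicated jump velocity updates CharacterMovement.
; Debug logic turns the healthbar toward the camera each tick and maps number keys to server weapon grants, async-loading weapon data if needed.
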(event EventBeginPlay
  ;[1 1 1] Begin Play - Setup Overhead Healthbar
  (|CallParentFunction)
  (bind _asw_overhead_health_bar (Utilities|Casting|CastToW_OverheadHealthBar (UserInterface|GetUserWidgetObject (Variables|Default|GetOverheadHealthBar))))
  (Default|SetupWidget _asw_overhead_health_bar self))

(event EventExecuteDeath
  ;[1 1 1] On Death Blueprint Implementation - TODO : Add Respawn Timers instead of just a static delay
  (|CallParentFunction))

(event EventFellOffWorld
  ;[1 1 1] Fall of World Event - If we hit a killfloor
  (|CallParentFunction)
  (GameplayEffects|ApplyGameplayEffectToSelf :self (Class|GEMCharacter|GetAbilitySystemComponent) :GameplayEffectClass "/Game/Blueprints/Game/GE/Misc/GE_InstantDeath.GE_InstantDeath_C"))

(event EventOnLanded
  (params (Hit :type Hit%20Result%20Structure%20%28by%20ref%29))
  ;[1 1 1] Fall Damage
  (CallFunction|FallDamage))

(event Custom|Server_AddToInventory
  (params (AssetID :type Primary%20Asset%20Id%20Structure))
  (bind _returnvalue (Class|KismetSystemLibrary|GetObjectfromPrimaryAssetId AssetID))
  (Utilities|IsValid _returnvalue
    (:Is%20Valid
      _)
    (:Is%20Not%20Valid
      (|AsyncLoadPrimaryAsset AssetID
        (:Completed
          _))))
  (bind _asgemweapon_data (Utilities|Casting|CastToGEMWeaponData _returnvalue))
  (Class|GEMCharacter|AddWeapontoInventory (Utilities|Struct|MakeInventoryWeaponData _asgemweapon_data 0 -1) true))

(event EventTick
  (params (DeltaSeconds :type Float%20%28single-precision%29))
  (bind _overheadhealthbar (Variables|Default|GetOverheadHealthBar))
  (|CallParentFunction DeltaSeconds)
  ;[0.2812 0.2812 0.2812] Hack together for rotating our Overhead Healthbar to where our player is looking
  (Utilities|FlowControl|Sequence
    (:then_0
      (Utilities|IsValid _overheadhealthbar
        (:Is%20Valid
          (Transformation|SetWorldRotation _overheadhealthbar (Math|Rotator|FindLookatRotation (Transformation|GetWorldLocation _overheadhealthbar) (Transformation|GetActorLocation (Game|GetPlayerCameraManager 0))) false false))))))

(event Input|KeyboardEvents|9
  (params (Key :type Key%20Structure :default "None"))
  (:Pressed
    (CallFunction|ServerAddtoInventory "Weapon:M4")))

(event Input|KeyboardEvents|7
  (params (Key :type Key%20Structure :default "None"))
  (:Pressed
    (CallFunction|ServerAddtoInventory "Weapon:Shotgun")))

(event Input|KeyboardEvents|6
  (params (Key :type Key%20Structure :default "None"))
  (:Pressed
    (CallFunction|ServerAddtoInventory "Weapon:SMG")))

(fn ConstructionScript)

(fn OnRepJumpVelocity
  (Variables|/Script/Engine.CharacterMovementComponent|SetJumpZVelocity (Variables|Character|GetCharacterMovement) (Variables|Default|GetJumpVelocity))
  (return))

(fn FallDamage
  (bind _output_get (LocalVariables|SetLocalFallDamage (Math|Curves|GetFloatValue (Variables|Default|GetFallDamageCurve) (.z (Transformation|GetVelocity)))))
  (if (not (Math|Float|NearlyEqual(Float) _output_get 0.0 1e-06))
    (bind _returnvalue (Ability|GameplayEffect|AssignTagSetbyCallerMagnitude (GameplayEffects|MakeOutgoingSpec :self (Class|GEMCharacter|GetAbilitySystemComponent) :GameplayEffectClass "/Game/Blueprints/Game/Debug/GE_FallDamage.GE_FallDamage_C") "(TagName=\"Data.Value1\")" (LocalVariables|GetLocalFallDamage)))
    (GameplayEffects|ApplyGameplayEffectSpecToSelf (Class|GEMCharacter|GetAbilitySystemComponent) _returnvalue)))