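; BP_Rifle is a rifle weapon Blueprint that sets up a render-to-texture scope sight for the player.
; After weapon data setup, if it uses scope scene capture and player 0 owns it, it creates a render target for the scope capture.
; A dynamic material made from the sight's element 1 receives that texture and is assigned to element 0.
; The construction script only calls its parent.
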(event EventPostSetupWeaponData
  (if (Class|GEMWeapon|UsesScopeSceneCapture)
    (if (== (Game|GetPlayerCharacter 0) (Components|GetOwner))
      (bind _returnvalue (Rendering|CreateRenderTarget2D 1024 1024 "RTF_RGBA16f"))
      (Variables|/Script/Engine.SceneCaptureComponent2D|SetTextureTarget (Class|GEMWeapon|GetScopeSceneCapture) _returnvalue)
      (bind _returnvalue_2 (Rendering|Material|CreateDynamicMaterialInstance (Class|GEMWeapon|GetSight) 1 0 "None" :!class /Script/Engine.PrimitiveComponent))
      (Rendering|Material|SetTextureParameterValue _returnvalue_2 "RenderTexture2D" (Variables|/Script/Engine.SceneCaptureComponent2D|GetTextureTarget (Class|GEMWeapon|GetScopeSceneCapture)))
      (Rendering|Material|SetMaterial (Class|GEMWeapon|GetSight) 0 _returnvalue_2))))

(fn ConstructionScript
  (|CallParentFunction))